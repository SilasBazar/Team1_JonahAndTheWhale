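; Crab enemy character for a side-scroller, with two overlap volumes that decide whether it hurts the player or dies.
; Overlapping the GiveDamage component subtracts one Health from the SideScrollerCharacter and plays a sound at the crab's location.
; Overlapping the TakeDamage component with that character plays a different sound and destroys the crab.
; No movement or AI logic lives in this graph.
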(event `self.GiveDamage.OnComponentBeginOverlap`
  (params (OverlappedComponent :type "PrimitiveComponent Object Reference") (OtherActor :type "Actor Object Reference") (OtherComp :type "PrimitiveComponent Object Reference") (OtherBodyIndex :type Integer) (bFromSweep :type Boolean) (SweepResult :type "HitResult Structure (by ref)"))
  (bind _asside_scroller_character (cast `/Game/SideScrollerBP/Blueprints/SideScrollerCharacter` OtherActor))
  (set `/Game/SideScrollerBP/Blueprints/SideScrollerCharacter.Health` (- (`/Game/SideScrollerBP/Blueprints/SideScrollerCharacter.Health` _asside_scroller_character) 1) _asside_scroller_character)
  (`GameplayStatics.PlaySoundAtLocation` "/Engine/EditorSounds/Notifications/CompileFailed.CompileFailed" (`self.K2_GetActorLocation`) (struct) 1.0 1.0 0.0 null null null))

(event `self.TakeDamage.OnComponentBeginOverlap`
  (params (OverlappedComponent :type "PrimitiveComponent Object Reference") (OtherActor :type "Actor Object Reference") (OtherComp :type "PrimitiveComponent Object Reference") (OtherBodyIndex :type Integer) (bFromSweep :type Boolean) (SweepResult :type "HitResult Structure (by ref)"))
  (cast `/Game/SideScrollerBP/Blueprints/SideScrollerCharacter` OtherActor)
  (`GameplayStatics.PlaySoundAtLocation` "/Engine/VREditor/Sounds/UI/Dockable_Window_Close.Dockable_Window_Close" (`self.K2_GetActorLocation`) (struct) 1.0 1.0 0.0 null null null)
  (`self.K2_DestroyActor`))

(fn `UserConstructionScript`)