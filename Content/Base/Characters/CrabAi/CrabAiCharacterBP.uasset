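; Crab enemy character for a side-scroller that hurts the player on contact and can be killed by the player.
; A GiveDamage overlap takes one health from the SideScrollerCharacter and plays a hit sound.
; A TakeDamage overlap with that character plays a sound, spawns the EnemyDied effect and destroys the crab.
; When PawnSensing sees a pawn while the crab moves quickly along Y, it plays a 2D walking sound.
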(event `self.PawnSensing.OnSeePawn`
  (params (Pawn :type "Pawn Object Reference"))
  (bind (_velocity_x _velocity_y) (`KismetMathLibrary.BreakVector` (`MovementComponent.Velocity` (`self.GetMovementComponent`))))
  (bind _returnvalue (or (> _velocity_y 100.0) (< _velocity_y -100.0)))
  (if _returnvalue
    (`GameplayStatics.PlaySoundAtLocation` null (0.0 0.0 0.0) (struct) 1.0 1.0 0.0 null null null)
    (`GameplayStatics.PlaySound2D` "/Game/Base/Characters/CrabAi/Audio/Untitled_5_02_1Music_for_whales__crab_walking_1.Untitled_5_02_1Music_for_whales__crab_walking_1" 5.0 1.0 254.0 null null _returnvalue)))

(event `self.GiveDamage.OnComponentBeginOverlap`
  (params (OverlappedComponent :type "PrimitiveComponent Object Reference") (OtherActor :type "Actor Object Reference") (OtherComp :type "PrimitiveComponent Object Reference") (OtherBodyIndex :type Integer) (bFromSweep :type Boolean) (SweepResult :type "HitResult Structure (by ref)"))
  (bind _asside_scroller_character (cast `/Game/SideScrollerBP/Blueprints/SideScrollerCharacter` OtherActor))
  (set `/Game/SideScrollerBP/Blueprints/SideScrollerCharacter.Health` (- (`/Game/SideScrollerBP/Blueprints/SideScrollerCharacter.Health` _asside_scroller_character) 1) _asside_scroller_character)
  (`GameplayStatics.PlaySoundAtLocation` "/Game/Base/Characters/CrabAi/Audio/Music_for_whales_11_01_25Music_for_whales__crab_hit_2.Music_for_whales_11_01_25Music_for_whales__crab_hit_2" (`self.K2_GetActorLocation`) (struct) 1.0 1.0 0.0 null null null))

(event `self.TakeDamage.OnComponentBeginOverlap`
  (params (OverlappedComponent :type "PrimitiveComponent Object Reference") (OtherActor :type "Actor Object Reference") (OtherComp :type "PrimitiveComponent Object Reference") (OtherBodyIndex :type Integer) (bFromSweep :type Boolean) (SweepResult :type "HitResult Structure (by ref)"))
  (cast `/Game/SideScrollerBP/Blueprints/SideScrollerCharacter` OtherActor)
  (`GameplayStatics.PlaySoundAtLocation` "/Engine/VREditor/Sounds/UI/Dockable_Window_Close.Dockable_Window_Close" (`self.K2_GetActorLocation`) (struct) 1.0 1.0 0.0 null null null)
  (`NiagaraFunctionLibrary.SpawnSystemAtLocation` "/Game/Base/Characters/CrabAi/EnemyDied.EnemyDied" (`self.K2_GetActorLocation`))
  (`self.K2_DestroyActor`))

(fn `UserConstructionScript`)