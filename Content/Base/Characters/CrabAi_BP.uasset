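; CrabAi_BP is a crab enemy that chases and damages the side-scroller player character.
; Pawn sensing drives an AI move toward the seen player; on success it subtracts health from the capsule hit's actor and plays a sound.
; A DamageTake flag inserts a delay before the next chase.
; Player overlap with DamageZone awards coins through AddCoins5X, plays a sound and destroys the crab.
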(event `self.PawnSensing.OnSeePawn`
  (params (Pawn :type "Pawn Object Reference"))
  (if (`self.DamageTake?`)
    (`KismetSystemLibrary.Delay` 3.0)
    (set `self.DamageTake?` false)
    (else
      (bind _asside_scroller_character (cast `/Game/SideScrollerBP/Blueprints/SideScrollerCharacter` Pawn))
      (`|AIMoveTo` self (0.0 0.0 0.0) _asside_scroller_character 1.0
        (:`OnSuccess`
          (set `self.DamageTake?` true)
          (bind _asside_scroller_character_2 (cast `/Game/SideScrollerBP/Blueprints/SideScrollerCharacter` (stale `self.CapsuleComponent.OnComponentHit` OtherActor)))
          (bind _output_get (set `/Game/SideScrollerBP/Blueprints/SideScrollerCharacter.Health` (- (`/Game/SideScrollerBP/Blueprints/SideScrollerCharacter.Health` _asside_scroller_character_2) 1) _asside_scroller_character_2))
          (`GameplayStatics.PlaySoundAtLocation` "/Engine/EditorSounds/Notifications/CompileFailed.CompileFailed" (`self.K2_GetActorLocation`) (struct) 1.0 1.0 0.0 null null null)
          (if (< _output_get 1)
            _))))))

(event `self.CapsuleComponent.OnComponentHit`
  (params (HitComponent :type "PrimitiveComponent Object Reference") (OtherActor :type "Actor Object Reference") (OtherComp :type "PrimitiveComponent Object Reference") (NormalImpulse :type "Vector Structure") (Hit :type "HitResult Structure (by ref)")))

(event `self.DamageZone.OnComponentBeginOverlap`
  (params (OverlappedComponent :type "PrimitiveComponent Object Reference") (OtherActor :type "Actor Object Reference") (OtherComp :type "PrimitiveComponent Object Reference") (OtherBodyIndex :type Integer) (bFromSweep :type Boolean) (SweepResult :type "HitResult Structure (by ref)"))
  (bind _asside_scroller_character (cast `/Game/SideScrollerBP/Blueprints/SideScrollerCharacter` OtherActor))
  (`/Game/SideScrollerBP/Blueprints/SideScrollerCharacter.AddCoins_5X` _asside_scroller_character)
  (`GameplayStatics.SpawnSoundAtLocation` "/Engine/VREditor/Sounds/UI/Dockable_Window_Close.Dockable_Window_Close" (`self.K2_GetActorLocation`) (struct) 1.0 1.0 0.0 null null)
  (`self.K2_DestroyActor`))

(fn `UserConstructionScript`)