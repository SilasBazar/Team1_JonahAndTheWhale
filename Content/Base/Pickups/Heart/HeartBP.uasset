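; Heart pickup Blueprint that restores health to the side-scroller player character on overlap.
; When its box collider overlaps a SideScrollerCharacter, it grants one health, then destroys itself.
; Before destruction it plays the collect sound and spawns a scaled-down Coin particle effect at its location.
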(event `self.Box.OnComponentBeginOverlap`
  (params (OverlappedComponent :type "PrimitiveComponent Object Reference") (OtherActor :type "Actor Object Reference") (OtherComp :type "PrimitiveComponent Object Reference") (OtherBodyIndex :type Integer) (bFromSweep :type Boolean) (SweepResult :type "HitResult Structure (by ref)"))
  (bind _asside_scroller_character (cast `/Game/SideScrollerBP/Blueprints/SideScrollerCharacter` OtherActor))
  (`/Game/SideScrollerBP/Blueprints/SideScrollerCharacter.GainHealth` _asside_scroller_character 1)
  (`self.HeartPlaySound`)
  (`self.K2_DestroyActor`))

(event `HeartPlaySound`
  (`GameplayStatics.PlaySoundAtLocation` "/Game/Base/Pickups/Heart/HeartCollect.HeartCollect" (`self.K2_GetActorLocation`) (struct) 1.0 1.0 0.0 null null null)
  (`NiagaraFunctionLibrary.SpawnSystemAtLocation` "/Game/Base/Pickups/Coin/Coin.Coin" (`self.K2_GetActorLocation`) (struct) (0.4 0.4 0.25)))

(fn `UserConstructionScript`)