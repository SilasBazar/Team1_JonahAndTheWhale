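; Key pickup for the stick altar that the side-scroller player collects by pressing Interact.
; An overlap volume enables input and opens a gate, which closes again when the overlap ends.
; A press through the open gate adds a key to the player character, flags the first stick key as obtained, plays a sound at the altar and destroys the actor.
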(event `InputAction|Interact`
  (params (Key :type "Key Structure"))
  (:`Pressed`
    (`/Engine/EditorBlueprintResources/StandardMacros.Gate` true :!label _label
      (:`Exit`
        (bind _asside_scroller_character (cast `/Game/SideScrollerBP/Blueprints/SideScrollerCharacter` (`GameplayStatics.GetPlayerCharacter` 0)))
        (`/Game/SideScrollerBP/Blueprints/SideScrollerCharacter.AddKeys` _asside_scroller_character)
        (set `/Game/SideScrollerBP/Blueprints/SideScrollerCharacter.GotStick1Key?` true _asside_scroller_character)
        (`GameplayStatics.PlaySoundAtLocation` "/Engine/VREditor/Sounds/VR_ungrab.VR_ungrab" (`SceneComponent.K2_GetComponentLocation` (`self.StickAlter`)) (struct) 1.0 1.0 0.0 null null null)
        (`self.K2_DestroyActor`)))))

(event `self.e.OnComponentBeginOverlap`
  (params (OverlappedComponent :type "PrimitiveComponent Object Reference") (OtherActor :type "Actor Object Reference") (OtherComp :type "PrimitiveComponent Object Reference") (OtherBodyIndex :type Integer) (bFromSweep :type Boolean) (SweepResult :type "HitResult Structure (by ref)"))
  (`self.EnableInput` (`GameplayStatics.GetPlayerController` 0))
  (goto _label :!via `Open`))

(event `self.e.OnComponentEndOverlap`
  (params (OverlappedComponent :type "PrimitiveComponent Object Reference") (OtherActor :type "Actor Object Reference") (OtherComp :type "PrimitiveComponent Object Reference") (OtherBodyIndex :type Integer))
  (goto _label :!via `Close`))

(fn `UserConstructionScript`)